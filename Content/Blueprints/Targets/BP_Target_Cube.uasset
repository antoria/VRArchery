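; Shooting target cube that slides back and forth between left and right limits and flashes green briefly when damaged.
; BeginPlay derives the limits from the start position along UnitVector and enables player input.
; Increase and decrease inputs shift it along DistanceVector, repeating once held past a short threshold.
; Each Tick rebuilds NextActorLocation from side movement and held distance input, then applies it without sweep.
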(event Game|Damage|EventAnyDamage
  (params (Damage :type Float%20%28single-precision%29) (DamageType :type Damage%20Type%20Object%20Reference) (InstigatedBy :type Controller%20Object%20Reference) (DamageCauser :type Actor%20Object%20Reference))
  ;[1 1 1] IsShot
  (Rendering|Material|SetMaterial (Variables|Default|GetStaticMesh) 0 "/Game/Materials/TargetMaterials/M_Targ_Green.M_Targ_Green")
  (Utilities|FlowControl|RetriggerableDelay 0.5)
  (Rendering|Material|SetMaterial (Variables|Default|GetStaticMesh) 0 "/Game/Medieval-Bows/Medieval93c8d5479024V1/data/Content/Medieval_Bows/Materials/M_Target_02.M_Target_02"))

(event EventTick
  (params (DeltaSeconds :type Float%20%28single-precision%29))
  ;[1 1 1] Tick
  (Variables|Default|SetNextActorLocation "0, 0, 0")
  (Utilities|FlowControl|Sequence
    (:then_0
      ;;[0 0.218 1] Automatic movement
      (if (Variables|Default|GetCanMove)
        (if (Variables|Default|GetGoingLeft)
          (if (> (Math|Vector|DotProduct (Transformation|GetActorLocation) (Variables|Default|GetUnitVector)) (Math|Vector|DotProduct (Variables|Default|GetMaxLeftPos) (Variables|Default|GetUnitVector)))
            (CallFunction|Move true)
            (else
              (bind _output_get (Variables|Default|SetGoingLeft false))
              (CallFunction|Move _output_get)))
          (elif (< (Math|Vector|DotProduct (Transformation|GetActorLocation) (Variables|Default|GetUnitVector)) (Math|Vector|DotProduct (Variables|Default|GetMaxRightPos) (Variables|Default|GetUnitVector)))
            (CallFunction|Move false)
            (else
              (bind _output_get_2 (Variables|Default|SetGoingLeft true))
              (CallFunction|Move _output_get_2))))))
    (:then_1
      ;;[0 1 0.0914] Distance update
      (if (Variables|Default|GetIncreasePressed)
        (Math|Float|CompareFloat (Class|PlayerController|GetInputKeyTimeDown (Game|GetPlayerController 0) (stale Input|ActionEvents|InputActionIncreaseTargetDistance Key)) 0.5
          (:>
            (CallFunction|ChangeActorDistance true)))))
    (:then_2
      (if (Variables|Default|GetDecreasePressed)
        (Math|Float|CompareFloat (Class|PlayerController|GetInputKeyTimeDown (Game|GetPlayerController 0) (stale Input|ActionEvents|InputActionDecreaseTargetDistance Key)) 0.5
          (:>
            (CallFunction|ChangeActorDistance false)))))
    (:then_3
      (Transformation|SetActorLocation (Variables|Default|GetNextActorLocation) false false))))

(event EventBeginPlay
  ;[1 1 1] Initialization
  (bind _output_get (Variables|Default|SetInitialPos (Transformation|GetActorLocation)))
  (Variables|Default|SetMaxLeftPos (- _output_get (* (Variables|Default|GetUnitVector) (Variables|Default|GetLeftDecal))))
  (Variables|Default|SetMaxRightPos (+ (Variables|Default|GetInitialPos) (* (Variables|Default|GetUnitVector) (Variables|Default|GetRightDecal))))
  (CallFunction|ChangeActorDistance true)
  (Input|EnableInput (Game|GetPlayerController 0)))

(event Input|ActionEvents|InputActionIncreaseTargetDistance
  (params (Key :type Key%20Structure))
  ;[1 1 1] Distance control
  (:Pressed
    (Variables|Default|SetIncreasePressed true)
    (CallFunction|ChangeActorDistance true))
  (:Released
    (Variables|Default|SetIncreasePressed false)))

(event Input|ActionEvents|InputActionDecreaseTargetDistance
  (params (Key :type Key%20Structure))
  ;[1 1 1] Distance control
  (:Pressed
    (Variables|Default|SetDecreasePressed true)
    (CallFunction|ChangeActorDistance false))
  (:Released
    (Variables|Default|SetDecreasePressed false)))

(fn ConstructionScript
  (|CallParentFunction))

(fn Move
  (params (GoingLeft :type Boolean))
  (if GoingLeft
    (Variables|Default|SetNextActorLocation (+ (- (Transformation|GetActorLocation) (* (Variables|Default|GetUnitVector) (Variables|Default|GetMoveSpeed))) (Variables|Default|GetNextActorLocation)))
    (else
      (Variables|Default|SetNextActorLocation (+ (+ (Transformation|GetActorLocation) (* (Variables|Default|GetUnitVector) (Variables|Default|GetMoveSpeed))) (Variables|Default|GetNextActorLocation))))))

(fn ChangeActorDistance
  (params (Increase :type Boolean))
  (if Increase
    (Variables|Default|SetNextActorLocation (+ (Variables|Default|GetNextActorLocation) (* (Variables|Default|GetDistanceVector) (Variables|Default|GetDistanceIncrement))))
    (else
      (Variables|Default|SetNextActorLocation (- (Variables|Default|GetNextActorLocation) (* (Variables|Default|GetDistanceVector) (Variables|Default|GetDistanceIncrement)))))))